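; BP_TextWriter is a Blueprint that exercises runtime localization by switching the current culture.
; On BeginPlay it steps through Russian, Spanish and English, pausing briefly between switches.
; After each switch it converts two Text variables to strings and prints them, showing how they resolve in that culture.
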(event `self.ReceiveBeginPlay`
  (`KismetInternationalizationLibrary.SetCurrentCulture` "ru")
  (`KismetSystemLibrary.PrintString` (`KismetTextLibrary.Conv_TextToString` (`self.Text`)) true true (struct :`G` 0.66 :`B` 1.0 :`A` 1.0) 10.0)
  (`KismetSystemLibrary.PrintString` (`KismetTextLibrary.Conv_TextToString` (`self.Text2`)) true true (struct :`G` 0.66 :`B` 1.0 :`A` 1.0) 10.0)
  (`KismetSystemLibrary.Delay` 2.0)
  (`KismetInternationalizationLibrary.SetCurrentCulture` "es")
  (`KismetSystemLibrary.PrintString` (`KismetTextLibrary.Conv_TextToString` (`self.Text`)) true true (struct :`G` 0.66 :`B` 1.0 :`A` 1.0) 10.0)
  (`KismetSystemLibrary.PrintString` (`KismetTextLibrary.Conv_TextToString` (`self.Text2`)) true true (struct :`G` 0.66 :`B` 1.0 :`A` 1.0) 10.0)
  (`KismetSystemLibrary.Delay` 2.0)
  (`KismetInternationalizationLibrary.SetCurrentCulture` "en")
  (`KismetSystemLibrary.PrintString` (`KismetTextLibrary.Conv_TextToString` (`self.Text`)) true true (struct :`G` 0.66 :`B` 1.0 :`A` 1.0) 10.0)
  (`KismetSystemLibrary.PrintString` (`KismetTextLibrary.Conv_TextToString` (`self.Text2`)) true true (struct :`G` 0.66 :`B` 1.0 :`A` 1.0) 10.0))

(fn `UserConstructionScript`)